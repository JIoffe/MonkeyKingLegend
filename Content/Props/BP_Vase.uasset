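; BP_Vase is a breakable vase prop that shatters when it takes any damage.
; On damage it turns off capsule physics and collision, then spawns a random handful of BP_VaseShard actors at randomly rotated points one capsule radius from its center, matching its scale.
; A dust cloud emitter plays at its location, and the vase destroys itself after a brief delay.
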(event Game|Damage|EventAnyDamage
  (params (Damage :type Float%20%28single-precision%29) (DamageType :type Damage%20Type%20Object%20Reference) (InstigatedBy :type Controller%20Object%20Reference) (DamageCauser :type Actor%20Object%20Reference))
  (bind _capsule (Variables|Default|GetCapsule))
  (Physics|SetSimulatePhysics _capsule false)
  (Collision|SetCollisionEnabled _capsule "NoCollision")
  (for _index (range 0 (Math|Random|RandomIntegerinRange 3 6))
    (Game|SpawnActorfromClass "/Game/FX/BP_VaseShard.BP_VaseShard_C" (Math|Transform|MakeTransform (+ (Transformation|GetActorLocation) (* (Math|Random|RandomUnitVector) (Variables|/Script/Engine.CapsuleComponent|GetCapsuleRadius (Variables|Default|GetCapsule)))) (Math|Conversions|RotationFromXVector (* (Math|Random|RandomUnitVector) 9e+01)) (Transformation|GetActorScale3D)) "Undefined" 0 0))
  (Effects|SpawnEmitteratLocation "/Game/FX/PS_DustCloud.PS_DustCloud" (Transformation|GetActorLocation))
  (Utilities|FlowControl|Delay 0.1)
  (Actor|DestroyActor))

(fn ConstructionScript)